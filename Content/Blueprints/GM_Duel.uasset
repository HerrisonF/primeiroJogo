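; Game mode for a quick-draw duel between a tanuki samurai and a toad samurai.
; Tick moves the phase from Intro to Wait, then after a random delay to Draw, broadcasting the change, showing an exclamation actor and starting a restart timer.
; A successful attack defeats the opponent and hides the exclamation.
; Separate functions mark the duel Finished or reset phase, elapsed time and both samurai.
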(event `self.ReceiveBeginPlay`
  (bind _returnvalue (`GameplayStatics.GetActorOfClass` "/Game/Blueprints/BP_Exclamation.BP_Exclamation_C"))
  (set `self.BPExclamationRef` _returnvalue)
  (bind _returnvalue_2 (`GameplayStatics.GetActorOfClass` "/Game/Blueprints/BP_Samurai_Tanuki.BP_Samurai_Tanuki_C"))
  (set `self.SamuraiPlayer` _returnvalue_2)
  (bind _returnvalue_3 (`GameplayStatics.GetActorOfClass` "/Game/Blueprints/BP_Samurai_Toad.BP_Samurai_Toad_C"))
  (set `self.SamuraiToad` _returnvalue_3))

(event `self.ReceiveTick`
  (params (DeltaSeconds :type "Float (single-precision)"))
  (set `self.elapsedTime` (+ DeltaSeconds (`self.elapsedTime`)))
  (switch `/Game/Blueprints/Enums/E_Phases` (`self.Phase`)
    (:`NewEnumerator0`
      (if (>= (`self.elapsedTime`) (`self.RoundStartTime`))
        (set `self.Phase` "NewEnumerator1")
        (`KismetSystemLibrary.Delay` (`KismetMathLibrary.RandomFloatInRange` (`self.mindrawDelay`) (`self.maxDrawDelay`)))
        (set `self.Phase` "NewEnumerator2")
        (`self.DrawPhaseStarted`)
        (`/Engine/EditorBlueprintResources/StandardMacros.IsValid` (`self.BPExclamationRef`)
          (:`Is Valid`
            (`/Game/Blueprints/BP_Exclamation.setVisibility` (`self.BPExclamationRef`) true)
            (`KismetSystemLibrary.K2_SetTimerDelegate` (`|CreateDelegate` :!event `Reset`) (`self.RestartDelay`)))
          (:`Is Not Valid`
            (`KismetSystemLibrary.PrintString` "Ponto de exclamção inválido")))))))

(fn `AttackedSucessfuly`
  (params (isPlayer :type Boolean))
  (if isPlayer
    (`/Game/Blueprints/BP_Samurai.Defeated` (`self.SamuraiToad`))
    (else
      (`/Game/Blueprints/BP_Samurai.Defeated` (`self.SamuraiPlayer`))))
  (`/Engine/EditorBlueprintResources/StandardMacros.IsValid` (`self.BPExclamationRef`)
    (:`Is Valid`
      (`/Game/Blueprints/BP_Exclamation.setVisibility` (`self.BPExclamationRef`) false))))

(fn `Reset`
  (set `self.Phase` "NewEnumerator0")
  (set `self.elapsedTime` 0.0)
  (`/Game/Blueprints/BP_Samurai.Reset` (`self.SamuraiPlayer`))
  (`/Game/Blueprints/BP_Samurai.Reset` (`self.SamuraiToad`)))

(fn `setGameFinished`
  (set `self.Phase` "NewEnumerator3"))

(fn `UserConstructionScript`)